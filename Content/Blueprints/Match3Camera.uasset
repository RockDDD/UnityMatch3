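; Match-3 camera Blueprint that scales its orthographic width to fit the viewport's aspect ratio.
; CheckViewport caches the GlobalGameInstance, waits for a non-zero viewport size, then calls UpdateCamera through a DoOnce.
; UpdateCamera derives OrthoWidth from DefaultFit's aspect, the viewport's and DesiredSize, then sets IsCameraSet.
; Its 4:3 branch currently yields the same width, and the event graph is empty.
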(event EventBeginPlay)

(event Collision|EventActorBeginOverlap
  (params (OtherActor :type Actor%20Object%20Reference)))

(event EventTick
  (params (DeltaSeconds :type Float%20%28single-precision%29)))

(fn ConstructionScript)

(fn UpdateCamera
  (bind _returnvalue (Viewport|GetViewportSize))
  (bind _returnvalue_2 (Viewport|GetViewportSize))
  (bind _defaultfit (Variables|Default|GetDefaultFit))
  (bind (_x _y) (Math|Vector2D|BreakVector2D _returnvalue))
  (bind (_x_2 _y_2) (Math|Vector2D|BreakVector2D _defaultfit))
  (bind (_x_3 _y_3) (Math|Vector2D|BreakVector2D _returnvalue_2))
  (bind _returnvalue_3 (/ _y_3 _x_3))
  (bind _returnvalue_4 (/ _y_2 _x_2))
  (bind _returnvalue_5 (/ _returnvalue_4 _returnvalue_3))
  (if (Math|Float|NearlyEqual(Float) (/ _x _y) 0.75 0.01)
    (Development|PrintString "4x3Engaged")
    (Variables|/Script/Engine.CameraComponent|SetOrthoWidth (Variables|CameraActor|GetCameraComponent) (* (* _returnvalue_5 1.0) (Variables|Default|GetDesiredSize)))
    (Variables|Default|SetisCameraSet true)
    (else
      (Variables|/Script/Engine.CameraComponent|SetOrthoWidth (Variables|CameraActor|GetCameraComponent) (* _returnvalue_5 (Variables|Default|GetDesiredSize)))
      (Variables|Default|SetisCameraSet true)))
  (Development|PrintString "Camera Size Was Updated ***"))

(fn CheckViewport
  (bind _returnvalue (Viewport|GetViewportSize))
  (bind (_x _y) (Math|Vector2D|BreakVector2D _returnvalue))
  (Variables|Default|GetStoredGameInstance
    (:then
      _)
    (:else
      (bind _asglobal_game_instance (Utilities|Casting|CastToGlobalGameInstance (Game|GetGameInstance)))
      (Variables|Default|SetStoredGameInstance _asglobal_game_instance)))
  (Utilities|FlowControl|Sequence
    (:then_1
      (if (and (!= _x 0.0) (!= _y 0.0))
        (Utilities|FlowControl|DoOnce false
          (:Completed
            (CallFunction|UpdateCamera)))))))